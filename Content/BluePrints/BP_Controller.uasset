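; Player controller for a base-building strategy game with battles, handling camera pan and zoom, UI screens, timed warnings and four resources.
; BeginPlay creates the widgets and restores army menu and resources from GI_PlayerData.
; Select input branches on ChoosenArmy and ChoosenBuild: deploy counted troops on BP_Beach, place buildings (only houses spawn, after a sphere-trace check), or box-trace-select units.
; Number keys trigger resource, barracks-upgrade and army-menu shortcuts.
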(event `Key|Nine`
  (params (Key :type "Key Structure"))
  (:`Pressed`
    (bind _outactors (`GameplayStatics.GetAllActorsOfClass` "/Game/BluePrints/Buildings/BP_BuildingJunYing.BP_BuildingJunYing_C"))
    (for _array_element _outactors
      (`|ExecutionSequence`
        (:`then_0`
          (`KismetSystemLibrary.PrintString` (`|GetEnumeratorNameAsString` (`/Game/BluePrints/Buildings/BP_BuildingHQ.Level` _array_element))))
        (:`then_1`
          (if (`self.ActorHasTag` _array_element "ON")
            (`/Game/BluePrints/Buildings/BP_BuildingJunYing.升级军营` _array_element)))))))

(event `Key|Zero`
  (params (Key :type "Key Structure"))
  (:`Pressed`
    (`self.进入军营`)))

(event `资源不足`
  (bind _lowresourceui (`self.LowResourceUI`))
  (`UserWidget.AddToViewport` _lowresourceui 1)
  (`KismetSystemLibrary.Delay` 2.0)
  (`Widget.RemoveFromParent` _lowresourceui))

(event `退出军营`
  (`Widget.RemoveFromParent` (`self.ArmyMenuUI`))
  (`UserWidget.AddToViewport` (`self.BuildUI`) 0))

(event `结束战斗`
  (`UserWidget.AddToViewport` (`self.MapUI`) 0)
  (`Widget.RemoveFromParent` (`self.FightingUI`))
  (`UserWidget.AddToViewport` (`self.MainUI`) 9))

(event `金币变化`
  (params (GoldChange :type Integer))
  (bind _output_get (set `self.GoldNUM` (+ GoldChange (`self.GoldNUM`))))
  (`/Game/UI/WBP_Main.更新金币` (`self.MainUI`) _output_get))

(event `未解锁`
  (bind _lowlevelui (`self.LowLevelUI`))
  (`UserWidget.AddToViewport` _lowlevelui 1)
  (`KismetSystemLibrary.Delay` 2.0)
  (`Widget.RemoveFromParent` _lowlevelui))

(event `资源更新`
  (params (g :type Integer) (w :type Integer) (s :type Integer) (i :type Integer))
  (`self.金币变化` g)
  (`self.木材变化` w)
  (`self.石材变化` s)
  (`self.钢材变化` i))

(event `进入军营`
  (bind _armymenuui (`self.ArmyMenuUI`))
  (`Widget.RemoveFromParent` (`self.BuildUI`))
  (`UserWidget.AddToViewport` _armymenuui 0)
  (`/Game/UI/WBP_ArmyMenu.更新最大位置` _armymenuui)
  (`Widget.RemoveFromParent` (`self.BuildMenuUI`)))

(event `开始战斗`
  (`Widget.RemoveFromParent` (`self.MainUI`))
  (`Widget.RemoveFromParent` (`self.MapUI`))
  (`UserWidget.AddToViewport` (`self.FightingUI`) 0)
  (`Widget.RemoveFromParent` (`self.BuildUI`)))

(event `木材变化`
  (params (WoodChange :type Integer))
  (bind _output_get (set `self.WoodNUM` (+ WoodChange (`self.WoodNUM`))))
  (`/Game/UI/WBP_Main.更新木材` (`self.MainUI`) _output_get))

(event `建筑上限`
  (bind _buildingmaxui (`self.BuildingMaxUI`))
  (`UserWidget.AddToViewport` _buildingmaxui 1)
  (`KismetSystemLibrary.Delay` 2.0)
  (`Widget.RemoveFromParent` _buildingmaxui))

(event `关闭地图`
  (`UserWidget.AddToViewport` (`self.BuildUI`) 0)
  (`Widget.RemoveFromParent` (`self.MapUI`)))

(event `Key|Two`
  (params (Key :type "Key Structure"))
  (:`Pressed`
    (`self.金币变化` 10)))

(event `关闭建造`
  (`UserWidget.AddToViewport` (`self.BuildUI`) 0)
  (`Widget.RemoveFromParent` (`self.BuildMenuUI`)))

(event `石材变化`
  (params (StoneChange :type Integer))
  (bind _output_get (set `self.StoneNUM` (+ StoneChange (`self.StoneNUM`))))
  (`/Game/UI/WBP_Main.更新石材` (`self.MainUI`) _output_get))

(event `打开地图`
  (`Widget.RemoveFromParent` (`self.ArmyMenuUI`))
  (`Widget.RemoveFromParent` (`self.BuildUI`))
  (`Widget.RemoveFromParent` (`self.BuildMenuUI`))
  (`UserWidget.AddToViewport` (`self.MapUI`) 0))

(event `军营上限`
  (bind _armymaxui (`self.ArmyMaxUI`))
  (`UserWidget.AddToViewport` _armymaxui 1)
  (`KismetSystemLibrary.Delay` 2.0)
  (`Widget.RemoveFromParent` _armymaxui))

(event `钢材变化`
  (params (IronChange :type Integer))
  (bind _output_get (set `self.IronNUM` (+ IronChange (`self.IronNUM`))))
  (`/Game/UI/WBP_Main.更新钢材` (`self.MainUI`) _output_get))

(event `打开建造`
  (bind _buildmenuui (`self.BuildMenuUI`))
  (`UserWidget.AddToViewport` _buildmenuui 0)
  (`/Game/UI/WBP_BuildMenu.更新建筑` _buildmenuui)
  (`Widget.RemoveFromParent` (`self.BuildUI`)))

(event `Key|Three`
  (params (Key :type "Key Structure"))
  (:`Pressed`
    (`self.石材变化` 10)))

(event `self.ReceiveBeginPlay`
  (set `self.bShowMouseCursor` true)
  (`EnhancedInputSubsystemInterface.AddMappingContext` (subsystem `EnhancedInputLocalPlayerSubsystem`) "/Game/Input/IMC_COC.IMC_COC" 0 (struct))
  (bind _returnvalue (`|CreateWidget` "/Game/UI/WBP_Main.WBP_Main_C"))
  (bind _output_get (set `self.MainUI` _returnvalue))
  (`UserWidget.AddToViewport` _output_get 9)
  (bind _returnvalue_2 (`|CreateWidget` "/Game/UI/WBP_Build.WBP_Build_C"))
  (bind _output_get_2 (set `self.BuildUI` _returnvalue_2))
  (`UserWidget.AddToViewport` _output_get_2 0)
  (bind _returnvalue_3 (`|CreateWidget` "/Game/UI/WBP_BuildMenu.WBP_BuildMenu_C"))
  (set `self.BuildMenuUI` _returnvalue_3)
  (bind _returnvalue_4 (`|CreateWidget` "/Game/UI/WBP_ArmyMenu.WBP_ArmyMenu_C"))
  (set `self.ArmyMenuUI` _returnvalue_4)
  (bind _returnvalue_5 (`|CreateWidget` "/Game/UI/WBP_Map.WBP_Map_C"))
  (set `self.MapUI` _returnvalue_5)
  (bind _returnvalue_6 (`|CreateWidget` "/Game/UI/WBP_Fighting.WBP_Fighting_C"))
  (set `self.FightingUI` _returnvalue_6)
  (bind _returnvalue_7 (`|CreateWidget` "/Game/UI/WBP_ArmyMax.WBP_ArmyMax_C"))
  (set `self.ArmyMaxUI` _returnvalue_7)
  (bind _returnvalue_8 (`|CreateWidget` "/Game/UI/WBP_BuildingMax.WBP_BuildingMax_C"))
  (set `self.BuildingMaxUI` _returnvalue_8)
  (bind _returnvalue_9 (`|CreateWidget` "/Game/UI/WBP_LowLevel.WBP_LowLevel_C"))
  (set `self.LowLevelUI` _returnvalue_9)
  (bind _returnvalue_10 (`|CreateWidget` "/Game/UI/WBP_LowResource.WBP_LowResource_C"))
  (set `self.LowResourceUI` _returnvalue_10)
  (bind _returnvalue_11 (`|CreateWidget` "/Game/UI/WBP_CantSet.WBP_CantSet_C"))
  (set `self.CantSetUI` _returnvalue_11)
  (`KismetSystemLibrary.Delay` 0.5)
  (bind _asgi_player_data (cast `/Game/BluePrints/GI_PlayerData` (`GameplayStatics.GetGameInstance`)))
  (bind (_mainui1 _armymenuui1 _gold _wood _stone _iron) (`/Game/BluePrints/GI_PlayerData.LoadData` _asgi_player_data))
  (`/Engine/EditorBlueprintResources/StandardMacros.IsValid` _armymenuui1
    (:`Is Valid`
      (`self.LoadData` null _armymenuui1 _gold _wood _stone _iron)
      (`KismetSystemLibrary.PrintString` "loaded")
      (message `/Game/UI/BPI/BPI_ArmyUpdate.ArmyUpdate` (`self.FightingUI`))
      (`self.资源更新` 0)
      (set `self.bEnableClickEvents` true))
    (:`Is Not Valid`
      (`KismetSystemLibrary.PrintString` "failed"))))

(event `EnhancedInput|/Game/Input/IA_Move`
  (params (ActionValue :type "Vector2D Structure") (ElapsedSeconds :type "Float (double-precision)") (TriggeredSeconds :type "Float (double-precision)") (InputAction :type "InputAction Object Reference" :default "/Game/Input/IA_Move.IA_Move"))
  (bind _returnvalue (`self.K2_GetPawn`))
  ; 相机移动
  (:`Triggered`
    (`self.K2_AddActorLocalOffset` _returnvalue (* ActionValue_X (`self.GetActorForwardVector` _returnvalue) (`self.CameraSensitivity`)) false false)
    (`self.K2_AddActorLocalOffset` _returnvalue (* ActionValue_Y (`self.GetActorRightVector` _returnvalue) (`self.CameraSensitivity`)) false false)))

(event `EnhancedInput|/Game/Input/IA_Zoom`
  (params (ActionValue :type "Float (double-precision)") (ElapsedSeconds :type "Float (double-precision)") (TriggeredSeconds :type "Float (double-precision)") (InputAction :type "InputAction Object Reference" :default "/Game/Input/IA_Zoom.IA_Zoom"))
  (bind _returnvalue (`self.GetComponentByClass` (`self.K2_GetPawn`) "/Script/Engine.SpringArmComponent"))
  ; 相机缩放
  (:`Triggered`
    (set `SpringArmComponent.TargetArmLength` (`KismetMathLibrary.FClamp` (+ (* ActionValue (`self.ZoomSensitivity`)) (`SpringArmComponent.TargetArmLength` _returnvalue)) 2000.0 30000.0) _returnvalue)))

(event `医师`
  (bind _fightingui (`self.FightingUI`))
  (bind _cantsetui (`self.CantSetUI`))
  (bind _yishinum (`/Game/UI/WBP_Fighting.YiShiNUM` _fightingui))
  ; 部署
  (if (> _yishinum 0)
    (set `/Game/UI/WBP_Fighting.YiShiNUM` (- _yishinum 1) _fightingui)
    (`|SpawnActorFromClass` "/Game/BluePrints/Unit/BP_YiShi.BP_YiShi_C" (`KismetMathLibrary.MakeTransform` (`self.ArmyLocation`)) "AdjustIfPossibleButAlwaysSpawn" "MultiplyWithRoot" null null)
    (else
      (`UserWidget.AddToViewport` _cantsetui 0)
      (`KismetSystemLibrary.Delay` 1.0)
      (`Widget.RemoveFromParent` _cantsetui))))

(event `棍棒手`
  (bind _fightingui (`self.FightingUI`))
  (bind _cantsetui (`self.CantSetUI`))
  (bind _gunbangshounum (`/Game/UI/WBP_Fighting.GunBangShouNUM` _fightingui))
  ; 部署
  (if (> _gunbangshounum 0)
    (set `/Game/UI/WBP_Fighting.GunBangShouNUM` (- _gunbangshounum 1) _fightingui)
    (`|SpawnActorFromClass` "/Game/BluePrints/Unit/BP_GunBangShou.BP_GunBangShou_C" (`KismetMathLibrary.MakeTransform` (`self.ArmyLocation`)) "AdjustIfPossibleButAlwaysSpawn" "MultiplyWithRoot" null null)
    (else
      (`UserWidget.AddToViewport` _cantsetui 0)
      (`KismetSystemLibrary.Delay` 1.0)
      (`Widget.RemoveFromParent` _cantsetui))))

(event `骑士`
  (bind _fightingui (`self.FightingUI`))
  (bind _cantsetui (`self.CantSetUI`))
  (bind _qishinum (`/Game/UI/WBP_Fighting.QiShiNUM` _fightingui))
  ; 部署
  (if (> _qishinum 0)
    (set `/Game/UI/WBP_Fighting.QiShiNUM` (- _qishinum 1) _fightingui)
    (`|SpawnActorFromClass` "/Game/BluePrints/Unit/BP_QiShi.BP_QiShi_C" (`KismetMathLibrary.MakeTransform` (`self.ArmyLocation`)) "AdjustIfPossibleButAlwaysSpawn" "MultiplyWithRoot" null null)
    (else
      (`UserWidget.AddToViewport` _cantsetui 0)
      (`KismetSystemLibrary.Delay` 1.0)
      (`Widget.RemoveFromParent` _cantsetui))))

(event `EnhancedInput|/Game/Input/IA_Select`
  (params (ActionValue :type Boolean) (ElapsedSeconds :type "Float (double-precision)") (TriggeredSeconds :type "Float (double-precision)") (InputAction :type "InputAction Object Reference" :default "/Game/Input/IA_Select.IA_Select"))
  (bind (_worldlocation _worlddirection) (`self.DeprojectMousePositionToWorld`))
  (bind _cantsetui (`self.CantSetUI`))
  ; 部署
  (:`Started`
    (if (`|EnumInequality` (`self.ChoosenArmy`) "NewEnumerator11")
      (if (`|EnumEquality` (`self.ChoosenBuild`) "NewEnumerator0")
        (bind (_outhit _returnvalue) (`KismetSystemLibrary.LineTraceSingle` :`Start` _worldlocation :`End` (+ _worldlocation (* _worlddirection 1000000.0)) :`TraceChannel` "TraceTypeQuery1" :`DrawDebugType` "Persistent"))
        (if _returnvalue
          (cast `/Game/BluePrints/BP_Beach` (`.HitActor` (`GameplayStatics.BreakHitResult` _outhit))
            (:`then`
              (`KismetSystemLibrary.PrintString` "Hello")
              (set `self.ArmyLocation` (`.Location` (`GameplayStatics.BreakHitResult` _outhit)))
              (switch `/Game/BluePrints/Enum/E_ChoosenArmy` (`self.ChoosenArmy`)
                (:`NewEnumerator0`
                  (`self.棍棒手`))
                (:`NewEnumerator1`
                  (`self.轻步兵`))
                (:`NewEnumerator2`
                  (`self.弓箭手`))
                (:`NewEnumerator3`
                  (`self.重步兵`))
                (:`NewEnumerator4`
                  (`self.医师`))
                (:`NewEnumerator5`
                  (`self.法师`))
                (:`NewEnumerator6`
                  (`self.狂战士`))
                (:`NewEnumerator7`
                  (`self.骑兵`))
                (:`NewEnumerator8`
                  (`self.骑士`))
                (:`NewEnumerator9`
                  (`self.投石车`))
                (:`NewEnumerator10`
                  (`self.炮车`))))
            (:`CastFailed`
              (`UserWidget.AddToViewport` _cantsetui 0)
              (`KismetSystemLibrary.Delay` 1.0)
              (`Widget.RemoveFromParent` _cantsetui)))
          (else
            (`KismetSystemLibrary.PrintString` "no")))))))

(event `EnhancedInput|/Game/Input/IA_Select`
  (params (ActionValue :type Boolean) (ElapsedSeconds :type "Float (double-precision)") (TriggeredSeconds :type "Float (double-precision)") (InputAction :type "InputAction Object Reference" :default "/Game/Input/IA_Select.IA_Select"))
  (bind _startlocation (`self.startLocation`))
  (bind _endlocation (`self.endLocation`))
  (bind (_bblockinghit _binitialoverlap _time _distance _location) (`GameplayStatics.BreakHitResult` (`self.GetHitResultUnderCursorByChannel` "TraceTypeQuery1")))
  (bind _returnvalue (`|EnumEquality` (`self.ChoosenArmy`) "NewEnumerator11"))
  (bind _returnvalue_2 (`|EnumEquality` (`self.ChoosenBuild`) "NewEnumerator0"))
  (bind _returnvalue_3 (/ (+ _startlocation _endlocation) 2.0))
  (:`Started`
    (if _returnvalue_2
      (if _returnvalue
        (set `self.startLocation` _location)
        (`KismetArrayLibrary.Array_Clear` (`self.selectedUnit`)))))
  (:`Completed`
    (if _returnvalue_2
      (if _returnvalue
        (set `self.endLocation` _location)
        (bind _outhits (`KismetSystemLibrary.BoxTraceMulti` :`Start` _returnvalue_3 :`End` _returnvalue_3 :`HalfSize` (`KismetMathLibrary.MakeVector` (`KismetMathLibrary.Abs` (/ (- (.x _startlocation) (.x _endlocation)) 2.0)) (`KismetMathLibrary.Abs` (/ (- (.y _startlocation) (.y _endlocation)) 2.0)) 300.0) :`TraceChannel` "TraceTypeQuery3" :`DrawDebugType` "ForDuration"))
        (for _array_element _outhits
          (bind _asbp_unit_base (cast `/Game/BluePrints/Unit/BP_UnitBase` (`.HitActor` (`GameplayStatics.BreakHitResult` _array_element))))
          (`KismetArrayLibrary.Array_Add` (`self.selectedUnit`) _asbp_unit_base))))))

(event `法师`
  (bind _fightingui (`self.FightingUI`))
  (bind _cantsetui (`self.CantSetUI`))
  (bind _fashinum (`/Game/UI/WBP_Fighting.FaShiNUM` _fightingui))
  ; 部署
  (if (> _fashinum 0)
    (set `/Game/UI/WBP_Fighting.FaShiNUM` (- _fashinum 1) _fightingui)
    (`|SpawnActorFromClass` "/Game/BluePrints/Unit/BP_FaShi.BP_FaShi_C" (`KismetMathLibrary.MakeTransform` (`self.ArmyLocation`)) "AdjustIfPossibleButAlwaysSpawn" "MultiplyWithRoot" null null)
    (else
      (`UserWidget.AddToViewport` _cantsetui 0)
      (`KismetSystemLibrary.Delay` 1.0)
      (`Widget.RemoveFromParent` _cantsetui))))

(event `投石车`
  (bind _fightingui (`self.FightingUI`))
  (bind _cantsetui (`self.CantSetUI`))
  (bind _toushichenum (`/Game/UI/WBP_Fighting.TouShiCheNUM` _fightingui))
  ; 部署
  (if (> _toushichenum 0)
    (set `/Game/UI/WBP_Fighting.TouShiCheNUM` (- _toushichenum 1) _fightingui)
    (`|SpawnActorFromClass` "/Game/BluePrints/Unit/BP_TouShiChe.BP_TouShiChe_C" (`KismetMathLibrary.MakeTransform` (`self.ArmyLocation`)) "AdjustIfPossibleButAlwaysSpawn" "MultiplyWithRoot" null null)
    (else
      (`UserWidget.AddToViewport` _cantsetui 0)
      (`KismetSystemLibrary.Delay` 1.0)
      (`Widget.RemoveFromParent` _cantsetui))))

(event `轻步兵`
  (bind _fightingui (`self.FightingUI`))
  (bind _cantsetui (`self.CantSetUI`))
  (bind _qingbubingnum (`/Game/UI/WBP_Fighting.QingBuBingNUM` _fightingui))
  ; 部署
  (if (> _qingbubingnum 0)
    (set `/Game/UI/WBP_Fighting.QingBuBingNUM` (- _qingbubingnum 1) _fightingui)
    (`|SpawnActorFromClass` "/Game/BluePrints/Unit/BP_QingBuBing.BP_QingBuBing_C" (`KismetMathLibrary.MakeTransform` (`self.ArmyLocation`)) "AdjustIfPossibleButAlwaysSpawn" "MultiplyWithRoot" null null)
    (else
      (`UserWidget.AddToViewport` _cantsetui 0)
      (`KismetSystemLibrary.Delay` 1.0)
      (`Widget.RemoveFromParent` _cantsetui))))

(event `狂战士`
  (bind _fightingui (`self.FightingUI`))
  (bind _cantsetui (`self.CantSetUI`))
  (bind _kuangzhanshinum (`/Game/UI/WBP_Fighting.KuangZhanShiNUM` _fightingui))
  ; 部署
  (if (> _kuangzhanshinum 0)
    (set `/Game/UI/WBP_Fighting.KuangZhanShiNUM` (- _kuangzhanshinum 1) _fightingui)
    (`|SpawnActorFromClass` "/Game/BluePrints/Unit/BP_KuangZhanShi.BP_KuangZhanShi_C" (`KismetMathLibrary.MakeTransform` (`self.ArmyLocation`)) "AdjustIfPossibleButAlwaysSpawn" "MultiplyWithRoot" null null)
    (else
      (`UserWidget.AddToViewport` _cantsetui 0)
      (`KismetSystemLibrary.Delay` 1.0)
      (`Widget.RemoveFromParent` _cantsetui))))

(event `炮车`
  (bind _fightingui (`self.FightingUI`))
  (bind _cantsetui (`self.CantSetUI`))
  (bind _paochenum (`/Game/UI/WBP_Fighting.PaoCheNUM` _fightingui))
  ; 部署
  (if (> _paochenum 0)
    (set `/Game/UI/WBP_Fighting.PaoCheNUM` (- _paochenum 1) _fightingui)
    (`|SpawnActorFromClass` "/Game/BluePrints/Unit/BP_JiaNongPaoZhanChe.BP_JiaNongPaoZhanChe_C" (`KismetMathLibrary.MakeTransform` (`self.ArmyLocation`)) "AdjustIfPossibleButAlwaysSpawn" "MultiplyWithRoot" null null)
    (else
      (`UserWidget.AddToViewport` _cantsetui 0)
      (`KismetSystemLibrary.Delay` 1.0)
      (`Widget.RemoveFromParent` _cantsetui))))

(event `弓箭手`
  (bind _fightingui (`self.FightingUI`))
  (bind _cantsetui (`self.CantSetUI`))
  (bind _gongjianshounum (`/Game/UI/WBP_Fighting.GongJianShouNUM` _fightingui))
  ; 部署
  (if (> _gongjianshounum 0)
    (set `/Game/UI/WBP_Fighting.GongJianShouNUM` (- _gongjianshounum 1) _fightingui)
    (`|SpawnActorFromClass` "/Game/BluePrints/Unit/BP_Archer.BP_Archer_C" (`KismetMathLibrary.MakeTransform` (`self.ArmyLocation`)) "AdjustIfPossibleButAlwaysSpawn" "MultiplyWithRoot" null null)
    (else
      (`UserWidget.AddToViewport` _cantsetui 0)
      (`KismetSystemLibrary.Delay` 1.0)
      (`Widget.RemoveFromParent` _cantsetui))))

(event `骑兵`
  (bind _fightingui (`self.FightingUI`))
  (bind _cantsetui (`self.CantSetUI`))
  (bind _qibingnum (`/Game/UI/WBP_Fighting.QiBingNUM` _fightingui))
  ; 部署
  (if (> _qibingnum 0)
    (set `/Game/UI/WBP_Fighting.QiBingNUM` (- _qibingnum 1) _fightingui)
    (`|SpawnActorFromClass` "/Game/BluePrints/Unit/BP_QiBing.BP_QiBing_C" (`KismetMathLibrary.MakeTransform` (`self.ArmyLocation`)) "AdjustIfPossibleButAlwaysSpawn" "MultiplyWithRoot" null null)
    (else
      (`UserWidget.AddToViewport` _cantsetui 0)
      (`KismetSystemLibrary.Delay` 1.0)
      (`Widget.RemoveFromParent` _cantsetui))))

(event `重步兵`
  (bind _fightingui (`self.FightingUI`))
  (bind _cantsetui (`self.CantSetUI`))
  (bind _zhongbubingnum (`/Game/UI/WBP_Fighting.ZhongBuBingNUM` _fightingui))
  ; 部署
  (if (> _zhongbubingnum 0)
    (set `/Game/UI/WBP_Fighting.ZhongBuBingNUM` (- _zhongbubingnum 1) _fightingui)
    (`|SpawnActorFromClass` "/Game/BluePrints/Unit/BP_ZhongBuBing.BP_ZhongBuBing_C" (`KismetMathLibrary.MakeTransform` (`self.ArmyLocation`)) "AdjustIfPossibleButAlwaysSpawn" "MultiplyWithRoot" null null)
    (else
      (`UserWidget.AddToViewport` _cantsetui 0)
      (`KismetSystemLibrary.Delay` 1.0)
      (`Widget.RemoveFromParent` _cantsetui))))

(event `EnhancedInput|/Game/Input/IA_Select`
  (params (ActionValue :type Boolean) (ElapsedSeconds :type "Float (double-precision)") (TriggeredSeconds :type "Float (double-precision)") (InputAction :type "InputAction Object Reference" :default "/Game/Input/IA_Select.IA_Select"))
  (bind (_worldlocation _worlddirection) (`self.DeprojectMousePositionToWorld`))
  (bind _buildlocation (`self.BuildLocation`))
  (bind _cantsetui (`self.CantSetUI`))
  (:`Started`
    (if (`|EnumInequality` (`self.ChoosenBuild`) "NewEnumerator0")
      (if (`|EnumEquality` (`self.ChoosenArmy`) "NewEnumerator11")
        (bind (_outhit _returnvalue) (`KismetSystemLibrary.LineTraceSingle` :`Start` _worldlocation :`End` (+ _worldlocation (* _worlddirection 1000000.0)) :`TraceChannel` "TraceTypeQuery1" :`DrawDebugType` "Persistent"))
        (if _returnvalue
          (set `self.BuildLocation` (`.Location` (`GameplayStatics.BreakHitResult` _outhit)))
          (switch `/Game/BluePrints/Enum/E_ChoosenBuilding` (`self.ChoosenBuild`)
            (:`NewEnumerator1`
              (bind (_outhit_2 _returnvalue_2) (`KismetSystemLibrary.SphereTraceSingleForObjects` :`Start` _buildlocation :`End` _buildlocation :`Radius` 520.0 :`ObjectTypes` (`|MakeArray` "ObjectTypeQuery3" :!type "EObjectTypeQuery Enum") :`DrawDebugType` "Persistent"))
              (`|ExecutionSequence`
                (:`then_0`
                  (cast `StaticMeshComponent` (`.HitComponent` (`GameplayStatics.BreakHitResult` _outhit_2))
                    (:`then`
                      (`UserWidget.AddToViewport` _cantsetui 0)
                      (`KismetSystemLibrary.Delay` 1.0)
                      (`Widget.RemoveFromParent` _cantsetui))
                    (:`CastFailed`
                      (`|SpawnActorFromClass` "/Game/BluePrints/Buildings/BP_BuildingHouse.BP_BuildingHouse_C" (`KismetMathLibrary.MakeTransform` (`self.BuildLocation`)) "AdjustIfPossibleButAlwaysSpawn" "MultiplyWithRoot" null null))))
                (:`then_1`
                  (if _returnvalue_2
                    (`KismetSystemLibrary.PrintString` "Hello")))))
            (:`NewEnumerator2`
              (`KismetSystemLibrary.PrintString` "2")))
          (else
            (`KismetSystemLibrary.PrintString` "no")))))))

(fn `LoadData`
  (params (MainUI :type "/Game/UI/WBP_Main Object Reference") (ArmyMenuUI :type "/Game/UI/WBP_ArmyMenu Object Reference") (gold :type Integer) (wood :type Integer) (stone :type Integer) (iron :type Integer))
  (set `self.ArmyMenuUI` ArmyMenuUI)
  (set `self.GoldNUM` gold)
  (set `self.WoodNUM` wood)
  (set `self.StoneNUM` stone)
  (set `self.IronNUM` iron)
  (return))

(fn `SaveData`
  (returns (MainUI1 :type "/Game/UI/WBP_Main Object Reference") (ArmyMenuUI1 :type "/Game/UI/WBP_ArmyMenu Object Reference") (gold :type Integer) (wood :type Integer) (stone :type Integer) (iron :type Integer))
  (return (`self.MainUI`) (`self.ArmyMenuUI`) (`self.GoldNUM`) (`self.WoodNUM`) (`self.StoneNUM`) (`self.IronNUM`)))

(fn `UserConstructionScript`)