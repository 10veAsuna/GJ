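; BP_CameraPawn is a camera pawn that holds the player's Wood and Stone resource counts and shows them on screen.
; On BeginPlay it creates the WBP_Main widget and adds it to the viewport.
; Every Tick it pushes both counts to the widget's message updates.
; A Wood++ event adds a fixed amount of wood, while Stone is only read here.
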(event `self.ReceiveBeginPlay`
  (bind _returnvalue (`|CreateWidget` "/Game/UI/WBP_Main.WBP_Main_C"))
  (bind _output_get (set `self.Main` _returnvalue))
  (`UserWidget.AddToViewport` _output_get 0))

(event `self.ReceiveTick`
  (params (DeltaSeconds :type "Float (single-precision)"))
  (bind _main (`self.Main`))
  (message `/Game/BluePrints/API/BPI_UI.UpdateWood` _main (`self.Wood`))
  (message `/Game/BluePrints/API/BPI_UI.UpdateStone` _main (`self.Stone`)))

(event `/Game/BluePrints/API/BPI_Btt.Wood++`
  (set `self.Wood` (+ (`self.Wood`) 10)))

(fn `UserConstructionScript`)