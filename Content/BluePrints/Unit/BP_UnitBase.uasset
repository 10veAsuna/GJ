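; Base unit Blueprint with health, damage and death animations, and an attack on enemy or target HQ buildings.
; AnyDamage lowers CurrentHP, while Tick turns the HP widget toward the camera, updates its bar and destroys the unit after death once IsDie is set.
; FindBuilding caches the nearest BP_BuildingHQ, whose HP AttackBuilding reduces directly in a delayed loop until depleted.
; FindResource is an empty stub.
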(event `self.ReceiveAnyDamage`
  (params (Damage :type "Float (single-precision)") (DamageType :type "DamageType Object Reference") (InstigatedBy :type "Controller Object Reference") (DamageCauser :type "Actor Object Reference"))
  (set `self.currentHP` (`KismetMathLibrary.FTrunc` (- (`self.currentHP`) Damage)))
  (if (not (`self.isDie`))
    (`SkeletalMeshComponent.PlayAnimation` (`self.Mesh`) (`self.damageAnim`) false)))

(event `self.ReceiveTick`
  (params (DeltaSeconds :type "Float (single-precision)"))
  (`SceneComponent.K2_SetWorldRotation` (`self.HP`) (`KismetMathLibrary.FindLookAtRotation` (`self.K2_GetActorLocation`) (`PlayerCameraManager.GetCameraLocation` (`GameplayStatics.GetPlayerCameraManager` 0))) false false)
  (`ProgressBar.SetPercent` (`/Game/UI/WBP_HP.health` (`self.As WBP HP`)) (`KismetMathLibrary.Conv_IntToDouble` (/ (`self.currentHP`) 100)))
  (if (`self.isDie`)
    (`SkeletalMeshComponent.PlayAnimation` (`self.Mesh`) (`self.dieAnim`) false)
    (`KismetSystemLibrary.Delay` 1.5)
    (`self.K2_DestroyActor`)))

(event `self.ReceiveBeginPlay`
  (bind _aswbp_hp (cast `/Game/UI/WBP_HP` (`WidgetComponent.GetWidget` (`self.HP`))))
  (set `self.As WBP HP` _aswbp_hp))

(event `/Game/BluePrints/API/BPI_AI.AttackBuilding`
  (bind _as_bp_building_hq (`self.As BP Building HQ`))
  (bind _currenthp (`/Game/BluePrints/Buildings/BP_BuildingHQ.currentHP` _as_bp_building_hq))
  (if (> _currenthp 0) :!label _label
    (set `/Game/BluePrints/Buildings/BP_BuildingHQ.currentHP` (- _currenthp (`self.damage`)) _as_bp_building_hq)
    (`KismetSystemLibrary.Delay` 2.0)
    (goto _label)))

(fn `FindBuilding`
  (returns (Building :type "/Game/BluePrints/Buildings/BP_BuildingHQ Object Reference"))
  (bind _outactors (`GameplayStatics.GetAllActorsOfClass` "/Game/BluePrints/Buildings/BP_BuildingHQ.BP_BuildingHQ_C"))
  (bind _asbp_building_hq (cast `/Game/BluePrints/Buildings/BP_BuildingHQ` (`.ReturnValue` (`GameplayStatics.FindNearestActor` (`self.K2_GetActorLocation`) _outactors))))
  (bind _output_get (set `self.As BP Building HQ` _asbp_building_hq))
  (return _output_get))

(fn `FindResource`
  (returns (Resource :type "/Game/BluePrints/Actor/BP_Resource Object Reference"))
  (return null))

(fn `UserConstructionScript`)