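; GI_PlayerData is a game instance-style store for player data, holding resource totals and UI references.
; SaveData copies the main UI, army menu UI and gold, wood, stone and iron amounts into member variables.
; LoadData returns those same variables, with no disk or SaveGame persistence in either function.
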(fn `LoadData`
  (returns (MainUI1 :type "/Game/UI/WBP_Main Object Reference") (ArmyMenuUI1 :type "/Game/UI/WBP_ArmyMenu Object Reference") (gold :type Integer) (wood :type Integer) (stone :type Integer) (iron :type Integer))
  (return (`self.MainUI`) (`self.ArmyMenuUI`) (`self.GoldNUM`) (`self.WoodNUM`) (`self.StoneNUM`) (`self.IronNUM`)))

(fn `SaveData`
  (params (MainUI :type "/Game/UI/WBP_Main Object Reference") (ArmyMenuUI :type "/Game/UI/WBP_ArmyMenu Object Reference") (gold :type Integer) (wood :type Integer) (stone :type Integer) (iron :type Integer))
  (set `self.MainUI` MainUI)
  (set `self.ArmyMenuUI` ArmyMenuUI)
  (set `self.GoldNUM` gold)
  (set `self.WoodNUM` wood)
  (set `self.StoneNUM` stone)
  (set `self.IronNUM` iron)
  (return))