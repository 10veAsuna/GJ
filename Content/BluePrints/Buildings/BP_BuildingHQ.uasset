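; BP_BuildingHQ is a headquarters building actor that takes damage and shows its health on a floating HP widget.
; BeginPlay caches the WBP_HP widget from the HP component.
; Every tick turns that component toward the player camera and refreshes the health bar from CurrentHP over MaxHP.
; AnyDamage subtracts damage from CurrentHP with truncation; no death handling is present.
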(event `self.ReceiveBeginPlay`
  (bind _aswbp_hp (cast `/Game/UI/WBP_HP` (`WidgetComponent.GetWidget` (`self.HP`))))
  (set `self.As WBP HP` _aswbp_hp))

(event `self.ReceiveTick`
  (params (DeltaSeconds :type "Float (single-precision)"))
  (`SceneComponent.K2_SetWorldRotation` (`self.HP`) (`KismetMathLibrary.FindLookAtRotation` (`self.K2_GetActorLocation`) (`PlayerCameraManager.GetCameraLocation` (`GameplayStatics.GetPlayerCameraManager` 0))) false false)
  (`ProgressBar.SetPercent` (`/Game/UI/WBP_HP.health` (`self.As WBP HP`)) (`KismetMathLibrary.Conv_IntToDouble` (/ (`self.currentHP`) (`self.maxHP`)))))

(event `self.ReceiveAnyDamage`
  (params (Damage :type "Float (single-precision)") (DamageType :type "DamageType Object Reference") (InstigatedBy :type "Controller Object Reference") (DamageCauser :type "Actor Object Reference"))
  (set `self.currentHP` (`KismetMathLibrary.FTrunc` (- (`self.currentHP`) Damage))))

(fn `UserConstructionScript`)