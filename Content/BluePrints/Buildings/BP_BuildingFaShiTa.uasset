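; Mage tower building (FaShiTa) that automatically damages the nearest BP_UnitBase inside its detection sphere.
; Tick turns the HP widget toward the camera and uses a Gongsu Delay to pace attacks on living units.
; AnyDamage updates the HP bar and, at zero, sets IsDie to stop attacks and hide the mesh.
; Friend-tagged overlaps are stored in an array that targeting ignores; the Attack function is empty.
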(event `self.ReceiveTick`
  (params (DeltaSeconds :type "Float (single-precision)"))
  (`SceneComponent.K2_SetWorldRotation` (`self.HP`) (`KismetMathLibrary.FindLookAtRotation` (`self.K2_GetActorLocation`) (`PlayerCameraManager.GetCameraLocation` (`GameplayStatics.GetPlayerCameraManager` 0))) false false)
  (`KismetSystemLibrary.Delay` (`self.gongsu`))
  (if (not (`self.isDie`))
    (bind _asbp_unit_base (cast `/Game/BluePrints/Unit/BP_UnitBase` (`.ReturnValue` (`GameplayStatics.FindNearestActor` (`self.K2_GetActorLocation`) (`PrimitiveComponent.GetOverlappingActors` (`self.Sphere`) "/Game/BluePrints/Unit/BP_UnitBase.BP_UnitBase_C")))))
    (if (not (`/Game/BluePrints/Unit/BP_UnitBase.isDie` _asbp_unit_base))
      (`self.攻击` _asbp_unit_base))))

(event `攻击`
  (params (DamagedActor :type "Actor Object Reference"))
  (`GameplayStatics.ApplyDamage` DamagedActor (`KismetMathLibrary.Conv_IntToDouble` (`self.attackDamage`)))
  (`KismetSystemLibrary.Delay` (`self.gongsu`)))

(event `self.ReceiveBeginPlay`
  (bind _aswbp_hp (cast `/Game/UI/WBP_HP` (`WidgetComponent.GetWidget` (`self.HP`))))
  (set `self.As WBP HP` _aswbp_hp)
  (message `/Game/BluePrints/API/BPI_UI.UpdateHP` (`self.As WBP HP`) (`KismetMathLibrary.Conv_IntToDouble` (`self.currentHP`)) (`KismetMathLibrary.Conv_IntToDouble` (`self.maxHP`))))

(event `self.ReceiveAnyDamage`
  (params (Damage :type "Float (single-precision)") (DamageType :type "DamageType Object Reference") (InstigatedBy :type "Controller Object Reference") (DamageCauser :type "Actor Object Reference"))
  (bind _returnvalue (`KismetMathLibrary.FTrunc` (- (`self.currentHP`) Damage)))
  (if (<= _returnvalue 0)
    (set `self.currentHP` 0)
    (set `self.isDie` true)
    (else
      (set `self.currentHP` _returnvalue)))
  (if (`self.isDie`)
    (message `/Game/BluePrints/API/BPI_UI.UpdateHP` (`self.As WBP HP`) (`KismetMathLibrary.Conv_IntToDouble` (`self.currentHP`)) (`KismetMathLibrary.Conv_IntToDouble` (`self.maxHP`)))
    (`SceneComponent.SetVisibility` (`self.StaticMesh`) false false)
    (else
      (message `/Game/BluePrints/API/BPI_UI.UpdateHP` (`self.As WBP HP`) (`KismetMathLibrary.Conv_IntToDouble` (`self.currentHP`)) (`KismetMathLibrary.Conv_IntToDouble` (`self.maxHP`))))))

(event `self.Sphere.OnComponentBeginOverlap`
  (params (OverlappedComponent :type "PrimitiveComponent Object Reference") (OtherActor :type "Actor Object Reference") (OtherComp :type "PrimitiveComponent Object Reference") (OtherBodyIndex :type Integer) (bFromSweep :type Boolean) (SweepResult :type "HitResult Structure (by ref)"))
  (if (`self.ActorHasTag` OtherActor "Friend")
    (bind _asbp_unit_base (cast `/Game/BluePrints/Unit/BP_UnitBase` OtherActor))
    (bind _output_get (set `self.As BP Unit Base` _asbp_unit_base))
    (`KismetArrayLibrary.Array_Add` (`self.As BP Unit Base_0`) _output_get)))

(fn `attack`
  (params (DamagedActor1 :type "Actor Object Reference")))

(fn `UserConstructionScript`
  (`parent.UserConstructionScript`))