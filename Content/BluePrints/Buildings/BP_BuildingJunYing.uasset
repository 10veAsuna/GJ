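; Barracks (军营) building Blueprint whose custom event 升级军营 upgrades the barracks.
; While the Level enum is below its cap, the event advances it one step and adds a fixed number of Positions, printing both new values.
; At the cap it only prints a placeholder message; BeginPlay, overlap and Tick are disabled stubs, and construction just calls the parent.
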(event `升级军营`
  (if (< (`self.Level`) 2)
    (bind _output_get (set `self.Level` (cast `/Game/BluePrints/Enum/E_Level` (+ (`self.Level`) 1))))
    (`KismetSystemLibrary.PrintString` (`|GetEnumeratorNameAsString` _output_get))
    (bind _output_get_2 (set `self.positions` (+ (`self.positions`) 4)))
    (`KismetSystemLibrary.PrintString` (`KismetStringLibrary.Conv_IntToString` _output_get_2))
    (else
      (`KismetSystemLibrary.PrintString` "Hello"))))

(fn `UserConstructionScript`
  (`parent.UserConstructionScript`))