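; BP_BuildingCaiShiChang is a quarry building that periodically produces stone for the player.
; BeginPlay starts a looping timer that fires the 生产 (production) event every few seconds.
; That event switches on the building's Level and passes a larger fixed stone amount at each higher tier to BP_Controller's 石材变化.
; The controller is looked up with GetActorOfClass on every production tick.
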(event `self.ReceiveBeginPlay`
  (`KismetSystemLibrary.K2_SetTimerDelegate` (delegate `生产`) 5.0 true))

(event `生产`
  (switch `/Game/BluePrints/Enum/E_Level` (`self.Level`)
    (:`NewEnumerator0`
      (bind _returnvalue (`GameplayStatics.GetActorOfClass` "/Game/BluePrints/BP_Controller.BP_Controller_C"))
      (`/Game/BluePrints/BP_Controller.石材变化` _returnvalue 100))
    (:`NewEnumerator1`
      (bind _returnvalue_2 (`GameplayStatics.GetActorOfClass` "/Game/BluePrints/BP_Controller.BP_Controller_C"))
      (`/Game/BluePrints/BP_Controller.石材变化` _returnvalue_2 140))
    (:`NewEnumerator2`
      (bind _returnvalue_3 (`GameplayStatics.GetActorOfClass` "/Game/BluePrints/BP_Controller.BP_Controller_C"))
      (`/Game/BluePrints/BP_Controller.石材变化` _returnvalue_3 200))))

(fn `UserConstructionScript`
  (`parent.UserConstructionScript`))